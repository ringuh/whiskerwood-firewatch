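; BP_MapLoad is a FireWatch mod loader actor that injects the WBP_FireWatch widget into the game's HUD.
; It polls every 0.25 seconds, even while paused, for a top-level PlayHud whose MToolbar has a valid parent.
; It adds the widget to that parent with canvas or overlay slot layout, falling back to the viewport after 30 seconds of real time.
; Ticking stops once the widget is added.
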(event `self.ReceiveBeginPlay`
  (`self.SetTickableWhenPaused` true)
  (`self.SetActorTickInterval` 0.25))

(event `self.ReceiveTick`
  (params (DeltaSeconds :type "Float (single-precision)"))
  (bind _returnvalue (`GameplayStatics.GetPlayerController` 0))
  (bind _foundwidgets (`WidgetBlueprintLibrary.GetAllWidgetsOfClass` "/Script/ProjectArco.PlayHud"))
  (bind _returnvalue_2 (`Widget.GetParent` (`PlayHud.m_toolbar` (`|GetArrayItem` _foundwidgets))))
  (if (`KismetSystemLibrary.IsValid` _returnvalue_2)
    (bind _returnvalue_3 (`|CreateWidget` "/Game/Mods/FireWatch/WBP_FireWatch.WBP_FireWatch_C" _returnvalue))
    (`PanelWidget.AddChild` _returnvalue_2 _returnvalue_3)
    (bind _returnvalue_4 (`WidgetLayoutLibrary.SlotAsCanvasSlot` _returnvalue_3))
    (if (`KismetSystemLibrary.IsValid` _returnvalue_4)
      (`CanvasPanelSlot.SetAnchors` _returnvalue_4 (struct :`Minimum` (0.0 0.0) :`Maximum` (1.0 1.0)))
      (`CanvasPanelSlot.SetOffsets` :`self` _returnvalue_4)
      (else
        (bind _returnvalue_5 (`WidgetLayoutLibrary.SlotAsOverlaySlot` _returnvalue_3))
        (`OverlaySlot.SetHorizontalAlignment` _returnvalue_5 "HAlign_Fill")
        (`OverlaySlot.SetVerticalAlignment` _returnvalue_5 "VAlign_Fill")))
    (`self.SetActorTickEnabled` false)
    (elif (> (`GameplayStatics.GetRealTimeSeconds`) 30.0)
      (bind _returnvalue_6 (`|CreateWidget` "/Game/Mods/FireWatch/WBP_FireWatch.WBP_FireWatch_C" _returnvalue))
      (`UserWidget.AddToViewport` _returnvalue_6 0)
      (`self.SetActorTickEnabled` false))))

(fn `UserConstructionScript`)